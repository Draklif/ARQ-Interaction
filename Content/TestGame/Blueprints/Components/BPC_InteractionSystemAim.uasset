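; Actor component that lets its owner aim at and interact with BPI_Interactable actors through press, hold or tap inputs.
; Each tick it traces from the owner along the camera's forward vector to set the active interactable, resetting progress when the target changes.
; A screen-space widget component created at BeginPlay shows WBP_Interaction at the target with hold or tap progress.
; Completed interactions turn the owner toward the target and message it through the interface.
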(event Custom|InteractWithActor
  (bind _active_interactable (CallFunction|GetActiveInteractable))
  (bind _returnvalue (Components|GetOwner))
  (Utilities|IsValid _active_interactable
    (:Is%20Valid
      (Transformation|SetActorRotation _returnvalue (Math|Rotator|MakeRotator 0.0 0.0 (.yaw (Math|Rotator|FindLookatRotation (Transformation|GetActorLocation _returnvalue) (CallFunction|GetActiveInteractableLocation)))))
      (Class|BPIInteractable|Interact(Message) _active_interactable _returnvalue))))

(event Custom|InteractionBegin
  (bind _active_interactable (CallFunction|GetActiveInteractable))
  (Utilities|IsValid _active_interactable
    (:Is%20Valid
      (bind _interaction_type (Class|BPIInteractable|GetInteractionType(Message) _active_interactable))
      (switch Utilities|FlowControl|Switch|SwitchonE_InteractionType _interaction_type
        (:NewEnumerator0
          (CallFunction|InteractwithActor)
          (CallFunction|InteractionOver))
        (:NewEnumerator1
          (EventDispatchers|BindEventtoOnInteractPressOngoing (EventDispatchers|CreateEvent :!event Custom|InteractionOngoing))
          (EventDispatchers|BindEventtoOnInteractEnded (delegate Custom|HoldEnd)))
        (:NewEnumerator2
          (CallFunction|InteractionTapOngoing))))))

(event Custom|InteractionTapOngoing
  (bind _result (Math|Integer|IncrementInt (Variables|Default|GetCurrentTapCount))
    (:%20%20
      (bind _value (Class|BPIInteractable|GetTapCount(Message) (CallFunction|GetActiveInteractable)))
      (if (<= _value _result)
        (CallFunction|InteractwithActor :!label _label)
        (CallFunction|InteractionOver)
        (else
          (bind _interactionwidgetref (Variables|Default|GetInteractionWidgetRef)
            (:then
              (Default|SetProgressPercent _interactionwidgetref (/ (Variables|Default|GetCurrentTapCount) _value))
              (if (>= (Variables|Default|GetCurrentTapCount) _value)
                (Variables|Default|SetCurrentTapCount 0)
                (goto _label)))
            (:else)))))))

(event Custom|HoldEnd
  (CallFunction|InteractionOver)
  (EventDispatchers|UnbindEventfromOnInteractEnded (delegate Custom|HoldEnd)))

(event Custom|InteractionOngoing
  (params (Elapsed%20Time :type Float%20%28double-precision%29))
  (bind _active_interactable (CallFunction|GetActiveInteractable))
  (Utilities|IsValid _active_interactable
    (:Is%20Valid
      (bind _holdduration (Class|BPIInteractable|GetHoldDuration(Message) _active_interactable))
      (bind _interactionwidgetref (Variables|Default|GetInteractionWidgetRef)
        (:then
          (Default|SetProgressPercent _interactionwidgetref (/ Elapsed%20Time _holdduration)))
        (:else
          _))
      (if (>= Elapsed%20Time _holdduration)
        (EventDispatchers|UnbindEventfromOnInteractPressOngoing (delegate Custom|InteractionOngoing))
        (CallFunction|InteractwithActor)
        (CallFunction|InteractionOver)))))

(event Custom|InteractionOver
  (Utilities|IsValid (CallFunction|GetActiveInteractable)
    (:Is%20Valid
      (bind _interactionwidgetref (Variables|Default|GetInteractionWidgetRef)
        (:then
          (Default|SetProgressPercent _interactionwidgetref 0.0))
        (:else)))))

(event EventBeginPlay
  (bind _returnvalue (Game|AddComponentbyClass (Components|GetOwner) "/Script/UMG.WidgetComponent" true))
  (Class|WidgetComponent|SetWidgetSpace _returnvalue "Screen")
  (Class|WidgetComponent|SetDrawSize _returnvalue "(X=32.000000,Y=32.000000)")
  (Variables|Default|SetInteractionWidget _returnvalue))

(event EventTick
  (params (DeltaSeconds :type Float%20%28single-precision%29))
  (bind _returnvalue (Components|GetOwner))
  (bind _returnvalue_2 (Game|GetPlayerCameraManager 0))
  (bind _returnvalue_3 (Transformation|GetActorLocation _returnvalue))
  (Utilities|IsValid _returnvalue_2
    (:Is%20Valid
      (bind (_outhit _returnvalue_4) (Collision|LineTraceByChannel _returnvalue_3 (+ _returnvalue_3 (* (Math|Vector|GetForwardVector (Camera|GetCameraRotation _returnvalue_2)) 5e+02)) "TraceTypeQuery1" false 0 "None"))
      (if _returnvalue_4
        (Utilities|IsInteractable (.HitActor (Collision|BreakHitResult _outhit))
          (:True
            (Utilities|IsPreviousInteractable (.HitActor (Collision|BreakHitResult _outhit))
              (:True
                (Variables|Default|SetActiveInteractable (.HitActor (Collision|BreakHitResult _outhit))))
              (:False
                (Variables|Default|SetActiveInteractable (.HitActor (Collision|BreakHitResult _outhit)))
                ;[0.15 0.15 0.15 0.5] End previous interactions
                (Variables|Default|SetCurrentTapCount 0 :!label _label)
                (Variables|Default|SetInteractionWidgetRef 0)
                (EventDispatchers|UnbindallEventsfromOnInteractPressOngoing)
                (CallFunction|InteractionOver))))
          (:False
            (Variables|Default|SetActiveInteractable 0 :!label _label_2)
            (goto _label)))
        (else
          (goto _label_2)))
      (CallFunction|RenderInteractionWidget))))

(fn GetActiveInteractable
  (return (Variables|Default|GetActiveInteractable)))

(fn GetActiveInteractableLocation
  (bind _active_interactable (CallFunction|GetActiveInteractable))
  (bind _location (Class|BPIInteractable|GetInteractionLocation(Message) _active_interactable))
  (return (Math|Vector|SelectVector (Transformation|GetActorLocation _active_interactable) _location (Class|KismetMathLibrary|EqualExactlyVectorVector _location "0, 0, 0"))))

(fn RenderInteractionWidget
  (bind _active_interactable (CallFunction|GetActiveInteractable))
  (bind _interactionwidget (Variables|Default|GetInteractionWidget))
  (Utilities|IsValid _active_interactable
    (:Is%20Valid
      (bind _interaction_type (Class|BPIInteractable|GetInteractionType(Message) _active_interactable))
      (Variables|Default|GetInteractionWidgetRef
        (:then
          _)
        (:else
          (bind _returnvalue (Game|ConstructObjectfromClass (Components|GetOwner) "/Game/TestGame/Blueprints/Widgets/WBP_Interaction.WBP_Interaction_C" _interaction_type))
          (bind _output_get (Variables|Default|SetInteractionWidgetRef _returnvalue))
          (UserInterface|SetWidget _interactionwidget _output_get)))
      (Transformation|SetWorldLocation _interactionwidget (CallFunction|GetActiveInteractableLocation) false false))
    (:Is%20Not%20Valid
      (UserInterface|SetWidget _interactionwidget 0))))