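; Inventory component that stores items as item-and-quantity slots in an array capped by InventorySize.
; AddItem loops while space remains, clamping quantities to MaxStack and returning leftovers, but appends slots even for matches and ignores the incoming item when none matches.
; Removal by ID or index decrements a slot or deletes it, returning true only on deletion.
; Helpers handle lookup and space checks; UseItem is an empty stub.
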(event EventBeginPlay)

(event EventTick
  (params (DeltaSeconds :type Float%20%28single-precision%29)))

(fn AddItem
  (params (Item%20Info :type S%20Item%20Info%20Structure) (Quantity :type Integer))
  (bind (_id _maxstack) (Utilities|Struct|BreakS_ItemInfo Item%20Info))
  (bind _inventory (Variables|Default|GetInventory))
  (bind (_found _item_slot) (Auxiliary|FindItemSlotbyID _id))
  (bind (_item _quantity) (Utilities|Struct|BreakS_ItemSlot _item_slot))
  (bind (_item_slot_2 _remaining) (Auxiliary|CalculateRemaining _item _quantity _maxstack))
  (LocalVariables|SetRemaining%20Items Quantity)
  (if (Auxiliary|HasSpace) :!label _label
    (if _found
      (Utilities|Array|Add _inventory (.Item%20Slot (Auxiliary|CalculateRemaining _item (+ (LocalVariables|GetRemaining%20Items) _quantity) _maxstack)))
      (LocalVariables|SetRemaining%20Items (.Remaining (Auxiliary|CalculateRemaining _item (+ (LocalVariables|GetRemaining%20Items) _quantity) _maxstack)))
      (else
        (Utilities|Array|Add _inventory _item_slot_2)
        (LocalVariables|SetRemaining%20Items _remaining)))
    (while (> (LocalVariables|GetRemaining%20Items) 0)
      (goto _label))
    (return 0)
    (else
      (return (LocalVariables|GetRemaining%20Items)))))

(fn HasItem
  (params (Item%20ID :type Name))
  (bind _array_element (Utilities|Array|ForEachLoopwithBreak (Variables|Default|GetInventory) :!label _label)
    (:LoopBody
      (if (== Item%20ID (.ID (Utilities|Struct|BreakS_ItemInfo (Utilities|Struct|BreakS_ItemSlot _array_element))))
        (LocalVariables|SetFound true)
        (goto _label Break)))
    (:Completed
      (return (LocalVariables|GetFound)))))

(fn RemoveItembyID
  (params (Item%20ID :type Name) (Quantity :type Integer))
  (bind (_found _item_slot _item_index) (Auxiliary|FindItemSlotbyID Item%20ID))
  (bind _inventory (Variables|Default|GetInventory))
  (bind (_item _quantity) (Utilities|Struct|BreakS_ItemSlot _item_slot))
  (bind _returnvalue (- _quantity Quantity))
  (if _found
    (if (<= _returnvalue 0)
      (Utilities|Array|RemoveIndex _inventory _item_index)
      (return true)
      (else
        (Utilities|Array|SetArrayElem _inventory _item_index (Utilities|Struct|MakeS_ItemSlot _item _returnvalue))
        (return false)))
    (else
      (return false))))

(fn RemoveItembyIndex
  (params (Index :type Integer) (Quantity :type Integer))
  (bind (_item_slot _found) (Auxiliary|FindItemSlotbyIndex Index))
  (bind _inventory (Variables|Default|GetInventory))
  (bind (_item _quantity) (Utilities|Struct|BreakS_ItemSlot _item_slot))
  (bind _returnvalue (- _quantity Quantity))
  (if _found
    (if (<= _returnvalue 0)
      (Utilities|Array|RemoveIndex _inventory Index)
      (return true)
      (else
        (Utilities|Array|SetArrayElem _inventory Index (Utilities|Struct|MakeS_ItemSlot _item _returnvalue))
        (return false)))
    (else
      (return false))))

(fn UseItem
  (params (Item%20Info :type S%20Item%20Info%20Structure)))

(fn FindItemSlotbyID
  (params (Item%20ID :type Name))
  (for (_array_element _array_index) (Variables|Default|GetInventory)
    (if (== Item%20ID (Utilities|Struct|BreakS_ItemInfo (Utilities|Struct|BreakS_ItemSlot _array_element)))
      (return true _array_element _array_index)))
  (return false "" 0))

(fn FindItemSlotbyIndex
  (params (Index :type Integer))
  (bind _inventory (Variables|Default|GetInventory))
  (if (< Index (Utilities|Array|Length _inventory))
    (return (Utilities|Array|Get(acopy) _inventory Index) true)
    (else
      (return "" false))))

(fn HasSpace
  (return (< (Utilities|Array|Length (Variables|Default|GetInventory)) (Variables|Default|GetInventorySize))))

(fn CalculateRemaining
  (params (Item :type S%20Item%20Info%20Structure) (Quantity :type Integer) (Max%20Quantity :type Integer))
  (if (> Quantity Max%20Quantity)
    (LocalVariables|SetNew%20Item%20Slot (Utilities|Struct|MakeS_ItemSlot Item Max%20Quantity))
    (LocalVariables|SetRem (- Quantity Max%20Quantity))
    (else
      (LocalVariables|SetNew%20Item%20Slot (Utilities|Struct|MakeS_ItemSlot Item Quantity))))
  (return (LocalVariables|GetNew%20Item%20Slot) (LocalVariables|GetRem)))