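; BP_Turret is a turret that automatically fires non-homing projectiles on a fixed timer.
; A looping timer started at BeginPlay spawns the configurable projectile class at the TurretShootPoint transform at the set interval.
; The turret binds to each projectile's hit dispatcher and sends the struck actor a TakeDamage message with a fixed, blockable damage payload.
; It has no targeting or aiming logic.
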(event Custom|Shoot
  (bind _returnvalue (Game|SpawnActorfromClass (Variables|Default|GetProjectileClass) (Transformation|GetWorldTransform (Variables|Default|GetTurretShootPoint)) "Undefined" "MultiplyWithRoot" self 0.0 5.0 5e+02 0 false 2e+03 0))
  (EventDispatchers|BindEventtoOnProjectileHit _returnvalue (delegate Custom|On%20Hit)))

(event Custom|On%20Hit
  (params (Other%20Actor :type Actor%20Object%20Reference) (Hit :type Hit%20Result%20Structure))
  (Class|BPIDamageable|TakeDamage(Message) Other%20Actor (Utilities|Struct|MakeS_DamageInfo 1e+01 "NewEnumerator2" "NewEnumerator0" false true)))

(event EventBeginPlay
  (Utilities|Time|SetTimerbyEvent (delegate Custom|Shoot) (Variables|Default|GetFrecuency) true))

(fn ConstructionScript)