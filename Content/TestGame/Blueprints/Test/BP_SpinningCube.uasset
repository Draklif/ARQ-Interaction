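; BP_SpinningCube is a test actor for a spinning cube that can be interacted with.
; It calls ToggleSpin five seconds after BeginPlay and prints a Spanish message when the OnFullRotation event fires; the rotation logic is not defined in these graphs.
; Interact destroys the actor, while the interaction getters return its location, the first enumerator type, and zero hold duration and tap count.
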(event EventBeginPlay
  (Utilities|FlowControl|Delay 5.0)
  (Class|SpinningCube|ToggleSpin))

(event EventOnFullRotation
  (Development|PrintString "Vuelta completa"))

(event EventInteract
  (params (Interactor :type Actor%20Object%20Reference))
  (Actor|DestroyActor))

(fn ConstructionScript)

(fn GetHoldDuration
  (return 0.0))

(fn GetInteractionLocation
  (return (Transformation|GetActorLocation)))

(fn GetInteractionType
  (return "NewEnumerator0"))

(fn GetTapCount
  (return 0))