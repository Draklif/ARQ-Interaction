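; BP_ProgressionListener is an actor that turns a matching progression event into a condition event message.
; On BeginPlay it binds to the game instance's OnProgressionEvent.
; When an event's step ID and action target match its own, it reports its configured condition type, target and amount back to the game instance through ReportEventMessage.
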(event Custom|ProgressionEvent
  (params (StepID :type Name) (ActionTarget :type Name))
  (if (and (== StepID (Variables|ListensTo|GetStepID)) (== ActionTarget (Variables|ListensTo|GetActionTarget)))
    (Class|BPIProgression|ReportEvent(Message) (Game|GetGameInstance) (Variables|Reports|GetConditionType) (Variables|Reports|GetConditionTarget) (Variables|Reports|GetConditionAmount) false)))

(event EventBeginPlay
  (EventDispatchers|BindEventtoOnProgressionEvent (CallFunction|GetMyGameInstance) (delegate Custom|ProgressionEvent)))

(fn ConstructionScript)