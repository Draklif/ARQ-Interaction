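; Trigger actor that links a box volume to the progression system to play cinematic Level Sequences.
; Player overlap with the box reports a condition event to the game instance.
; A progression event with a matching ActionTarget locks look or move input per CameraInputMode, plays the sequence and hides the main HUD.
; When playback finishes, the game instance returns to the player and the HUD reappears; a FadeIn camera helper is defined but unused.
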(event OnComponentBeginOverlap(Box)
  (params (OverlappedComponent :type Primitive%20Component%20Object%20Reference) (OtherActor :type Actor%20Object%20Reference) (OtherComp :type Primitive%20Component%20Object%20Reference) (OtherBodyIndex :type Integer) (bFromSweep :type Boolean) (SweepResult :type Hit%20Result%20Structure%20%28by%20ref%29))
  (if (== OtherActor (Game|Player|GetPlayerPawn 0))
    (Class|BPIProgression|ReportEvent(Message) (Game|GetGameInstance) "NewEnumerator3" (Variables|Default|GetConditionTarget) 0 true)))

(event Custom|TryPlaySequence
  (params (StepID :type Name) (ActionTarget :type Name))
  (bind _returnvalue (Game|GetPlayerController 0))
  (if (== ActionTarget (Variables|Default|GetActionTarget))
    (Utilities|FlowControl|Sequence
      (:then_0
        (switch Utilities|FlowControl|Switch|SwitchonE_CameraInputMode (Variables|Default|GetCamera%20Input%20Mode)
          (:NewEnumerator1
            _)
          (:NewEnumerator2
            (Input|SetIgnoreMoveInput _returnvalue true)))
        (Input|SetIgnoreLookInput _returnvalue true))
      (:then_1
        (bind _levelsequenceplayer (CallFunction|PlaySequence))
        (EventDispatchers|BindEventtoOnFinished _levelsequenceplayer (delegate Custom|TryFinishSequence))
        (Class|BPIWidgetManager|HideWidget(Message) (HUD|GetHUD (Game|GetPlayerController 0)) "MainHUD")))))

(event Custom|TryFinishSequence
  (Class|BPICameraManager|ReturntoPlayer(Message) (Game|GetGameInstance) 0.0)
  (Class|BPIWidgetManager|ShowWidget(Message) (HUD|GetHUD (Game|GetPlayerController 0)) "MainHUD"))

(event EventBeginPlay
  (EventDispatchers|BindEventtoOnProgressionEvent (CallFunction|GetMyGameInstance) (delegate Custom|TryPlaySequence)))

(fn ConstructionScript)

(fn PlaySequence
  (bind _returnvalue (Sequencer|Player|CreateLevelSequencePlayer (Variables|Default|GetLevel%20Sequence)))
  (Sequencer|Player|Play _returnvalue :!class /Script/MovieScene.MovieSceneSequencePlayer)
  (return _returnvalue))