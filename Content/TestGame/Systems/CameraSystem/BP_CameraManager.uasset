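; BP_CameraManager is a camera manager that switches the player's view between registered cameras and the player pawn.
; RegisterCamera stores cameras in a map by ID, and SwitchToCamera looks one up and cubic-blends the first player controller's view target to it.
; ReturnToPlayer blends back to the pawn over a given time.
; On BeginPlay it registers itself with the game instance and binds to its progression event, whose handler is currently empty.
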(event Custom|ProgressionEvent
  (params (StepID :type Name) (ActionTarget :type Name)))

(event EventBeginPlay
  (bind _game_instance (CallFunction|GetMyGameInstance))
  (EventDispatchers|BindEventtoOnProgressionEvent _game_instance (delegate Custom|ProgressionEvent))
  (Class|BPICameraManager|SetCameraManager(Message) _game_instance self))

(fn ConstructionScript)

(fn SwitchtoCamera
  (params (CameraID :type Name) (BlendTime :type Float%20%28single-precision%29))
  (bind _cameras (Variables|Default|GetCameras))
  (bind (_value _returnvalue) (Utilities|Map|Find _cameras CameraID))
  (if _returnvalue
    (Game|Player|SetViewTargetwithBlend (Game|GetPlayerController 0) _value BlendTime "VTBlend_Cubic" 0.0 false)))

(fn ReturntoPlayer
  (params (BlendTime :type Float%20%28single-precision%29))
  (Game|Player|SetViewTargetwithBlend (Game|GetPlayerController 0) (Game|Player|GetPlayerPawn 0) BlendTime "VTBlend_Cubic" 0.0 false))

(fn RegisterCamera
  (params (CameraID :type Name%20%28by%20ref%29) (Camera :type Actor%20Object%20Reference%20%28by%20ref%29))
  (Utilities|Map|Add (Variables|Default|GetCameras) CameraID Camera))